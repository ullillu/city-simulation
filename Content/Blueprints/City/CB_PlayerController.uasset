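; Player controller for the city builder that relays camera input to the CB_CameraController pawn and handles building placement.
; OnPlacementInfoUpdated sets the building class and toggles placement mode, spawning a preview actor far below the world with an added AC_CityBuilder component.
; Each tick, a cursor trace moves the preview to the hit point.
; Left click spawns the building there if the component reports valid placement, then exits placement mode.
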(event Custom|OnPlacementInfoUpdated
  (params (InPlaceableActorType :type BP%20Placeable%20Item%20Class%20Reference) (InPlacebleMode :type Boolean))
  (bind _placeableactor (Variables|Default|GetPlaceableActor))
  (Variables|Default|SetPlaceableActorType InPlaceableActorType)
  (bind _output_get (Variables|Default|SetPlacableBuildingType InPlacebleMode))
  (if _output_get
    (Utilities|IsValid _placeableactor
      (:Is%20Valid
        (Actor|DestroyActor _placeableactor))
      (:Is%20Not%20Valid
        _))
    (CallFunction|RefreshPlaceableBuilding)
    (CallFunction|SetPlacementModeEnabled true)
    (else
      (CallFunction|SetPlacementModeEnabled false))))

(event EventTick
  (params (DeltaSeconds :type Float%20%28single-precision%29))
  (if (Variables|Default|GetPlacementModeEnabled)
    (CallFunction|UpdatePlacement)))

(event Input|ActionEvents|InputActionCameraZoomIn
  (params (Key :type Key%20Structure))
  (:Pressed
    (bind _ascb_camera_controller (Utilities|Casting|CastToCB_CameraController (Pawn|GetControlledPawn)))
    (Default|CameraZoom _ascb_camera_controller -1.0)))

(event Input|ActionEvents|InputActionCameraZoomOut
  (params (Key :type Key%20Structure))
  (:Pressed
    (bind _ascb_camera_controller (Utilities|Casting|CastToCB_CameraController (Pawn|GetControlledPawn)))
    (Default|CameraZoom _ascb_camera_controller 1.0)))

(event Input|ActionEvents|InputActionMouseLeftClick
  (params (Key :type Key%20Structure))
  (:Pressed
    (if (Variables|Default|GetPlacementModeEnabled)
      (CallFunction|SpawnBuilding))))

(event Input|AxisEvents|InputAxisCameraOrbit
  (params (AxisValue :type Float%20%28single-precision%29))
  (bind _ascb_camera_controller (Utilities|Casting|CastToCB_CameraController (Pawn|GetControlledPawn)))
  (Default|CameraOrbit _ascb_camera_controller AxisValue))

(event Input|AxisEvents|InputAxisMoveForward/Back
  (params (AxisValue :type Float%20%28single-precision%29))
  (bind _ascb_camera_controller (Utilities|Casting|CastToCB_CameraController (Pawn|GetControlledPawn)))
  (Default|MoveForward/Backward _ascb_camera_controller AxisValue))

(event Input|AxisEvents|InputAxisMoveLeft/Right
  (params (AxisValue :type Float%20%28single-precision%29))
  (bind _ascb_camera_controller (Utilities|Casting|CastToCB_CameraController (Pawn|GetControlledPawn)))
  (Default|MoveLeft/Right _ascb_camera_controller AxisValue))

(fn ConstructionScript)

(fn SetPlacementModeEnabled
  (params (Is%20Enabled :type Boolean))
  (bind _placeableactor (Variables|Default|GetPlaceableActor))
  (if (== Is%20Enabled (Variables|Default|GetPlacementModeEnabled))
    (return)
    (else
      (bind _output_get (Variables|Default|SetPlacementModeEnabled Is%20Enabled))
      (if _output_get
        (CallFunction|RefreshPlaceableBuilding)
        (else
          (Utilities|IsValid _placeableactor
            (:Is%20Valid
              (Actor|DestroyActor _placeableactor))))))))

(fn UpdatePlacement
  (bind (_worldlocation _worlddirection) (Game|Player|ConvertMouseLocationToWorldSpace))
  (bind _outhit (Collision|LineTraceByChannel _worldlocation (+ _worldlocation (* _worlddirection 10000)) "TraceTypeQuery3" false 0 "None"))
  (if (.bBlockingHit (Collision|BreakHitResult _outhit))
    (Transformation|SetActorLocation (Variables|Default|GetPlaceableActor) (.Location (Collision|BreakHitResult _outhit)) false false)))

(fn SpawnBuilding
  (bind _placeableactor (Variables|Default|GetPlaceableActor))
  (bind _returnvalue (Actor|GetComponentbyClass _placeableactor "/Game/Blueprints/City/Road/CityBuilder/AC_CityBuilder.AC_CityBuilder_C"))
  (Utilities|IsValid _returnvalue
    (:Is%20Valid
      (if (Variables|/Game/Blueprints/City/Road/CityBuilder/AC_CityBuilder.AC_CityBuilder_C|GetIsPlacementValid _returnvalue)
        (Game|SpawnActorfromClass (Variables|Default|GetPlaceableActorType) (Transformation|GetActorTransform (Variables|Default|GetPlaceableActor)) "AlwaysSpawn" 0 0)
        (CallFunction|SetPlacementModeEnabled false)))))

(fn RefreshPlaceableBuilding
  (bind _returnvalue (Game|SpawnActorfromClass (Variables|Default|GetPlaceableActorType) (Math|Transform|MakeTransform "0.000000,0.000000,-100000.000000") "AlwaysSpawn" 0 0))
  (bind _output_get (Variables|Default|SetPlaceableActor _returnvalue))
  (AddComponent|AddACCityBuilder _output_get))