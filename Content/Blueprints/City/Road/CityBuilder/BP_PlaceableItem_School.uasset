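; School placeable item for the city builder that previews which buildings it serves.
; HighlightArea scans every BP_Building by distance: near ones turn positive and are flagged as assigned to a school, while unassigned ones in an outer band turn negative and show their widget.
; UnhighlightArea restores the default material and hides widgets on all buildings, leaving the assignment flag set.
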(event EventBeginPlay
  (|CallParentFunction) ; This node is disabled and will not be called.\nDrag off pins to build functionality.
)

(event Collision|EventActorBeginOverlap
  (params (OtherActor :type Actor%20Object%20Reference))
  (|CallParentFunction OtherActor) ; This node is disabled and will not be called.\nDrag off pins to build functionality.
)

(event EventTick
  (params (DeltaSeconds :type Float%20%28single-precision%29))
  (|CallParentFunction DeltaSeconds) ; This node is disabled and will not be called.\nDrag off pins to build functionality.
)

(event EventHighlightArea
  (bind _outactors (Actor|GetAllActorsOfClass "/Game/Blueprints/City/Building/BP_Building.BP_Building_C"))
  (for _array_element _outactors
    (if (< (Math|Vector|VectorLength (- (Transformation|GetWorldLocation (Variables|Default|GetStaticMesh)) (Transformation|GetWorldLocation (Variables|/Game/Blueprints/City/Building/BP_Building.BP_Building_C|GetBuilding _array_element)))) 3e+02)
      (Rendering|Material|SetMaterial (Variables|/Game/Blueprints/City/Building/BP_Building.BP_Building_C|GetBuilding _array_element) 0 "/Game/Blueprints/City/Building/M_Positive.M_Positive")
      (Variables|/Game/Blueprints/City/Building/BP_Building.BP_Building_C|SetIsAssignedToSchool? _array_element true)
      (bind _ref (Default|GetWidgetRef _array_element))
      (Development|SetHiddeninGame _ref true false)
      (elif (< (Math|Vector|VectorLength (- (Transformation|GetWorldLocation (Variables|Default|GetStaticMesh)) (Transformation|GetWorldLocation (Variables|/Game/Blueprints/City/Building/BP_Building.BP_Building_C|GetBuilding _array_element)))) 5e+02)
        (if (Variables|/Game/Blueprints/City/Building/BP_Building.BP_Building_C|GetIsAssignedToSchool? _array_element)
          (bind _ref_2 (Default|GetWidgetRef _array_element))
          (Development|SetHiddeninGame _ref_2 true false)
          (else
            (Rendering|Material|SetMaterial (Variables|/Game/Blueprints/City/Building/BP_Building.BP_Building_C|GetBuilding _array_element) 0 "/Game/Blueprints/City/Building/M_Negative.M_Negative")
            (bind _ref_3 (Default|GetWidgetRef _array_element))
            (Development|SetHiddeninGame _ref_3 false false)))))))

(event EventUnhighlightArea
  (bind _outactors (Actor|GetAllActorsOfClass "/Game/Blueprints/City/Building/BP_Building.BP_Building_C"))
  (for _array_element _outactors
    (Rendering|Material|SetMaterial (Variables|/Game/Blueprints/City/Building/BP_Building.BP_Building_C|GetBuilding _array_element) 0 "/Game/Meshes/NEW_CityModel/M_Building.M_Building")
    (bind _ref (Default|GetWidgetRef _array_element))
    (Development|SetHiddeninGame _ref true false)))

(fn ConstructionScript
  (|CallParentFunction))